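; ObstacleSpreadBP is an animated obstacle with four static meshes that slide back and forth while spinning.
; Tick accumulates elapsed time and sets each mesh's relative Y from an offset sine wave, oscillating between 0 and 100 units from its parent's origin.
; Each mesh also gains a fixed local rotation step every frame, so spin speed depends on frame rate.
; A time-based absolute rotation node is left unconnected.
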(event EventBeginPlay)

(event Collision|EventActorBeginOverlap
  (params (OtherActor :type Actor%20Object%20Reference)))

(event EventTick
  (params (DeltaSeconds :type Float%20%28single-precision%29))
  (Variables|Default|SetcurrentTime (+ DeltaSeconds (Variables|Default|GetcurrentTime)))
  (for _array_element (Utilities|Array|MakeArray (Variables|Default|GetStaticMesh) (Variables|Default|GetStaticMesh1) (Variables|Default|GetStaticMesh2) (Variables|Default|GetStaticMesh3))
    (Transformation|SetRelativeLocation _array_element (Math|Vector|MakeVector 0.0 (* (+ (Math|Trig|Sin(Radians) (Variables|Default|GetcurrentTime)) 1.0) 5e+01) 0.0) false false)
    (Transformation|AddLocalRotation _array_element "1.000000, 0, 0" false false)))

(fn ConstructionScript)