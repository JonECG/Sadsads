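; Tube crawler actor that drives a camera rig following it along a Tube.
; Its construction script detaches CameraFrom and CameraTo, which Tick places on the tube's center axis behind and ahead of the crawler's RelativePosition.
; As those points fall out of line with the actor, CameraFrom shifts partly toward CameraTo's mirror point through the actor.
; CameraFrom looks at CameraTo, taking its up vector from the tube orientation at the crawler.
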(event EventBeginPlay)

(event Collision|EventActorBeginOverlap
  (params (OtherActor :type Actor%20Object%20Reference)))

(event EventTick
  (params (DeltaSeconds :type Float%20%28single-precision%29))
  (bind _returnvalue (Transformation|GetActorLocation))
  (bind _tube (Variables|Default|Gettube))
  (bind _cameraseparation (Variables|Default|GetCameraSeparation))
  (bind _relativeposition (Variables|Default|GetrelativePosition))
  (bind _z (Math|Vector|BreakVector _relativeposition))
  (bind _returnvalue_2 (- _z _cameraseparation))
  (bind _returnvalue_3 (+ _cameraseparation _z))
  (bind _returnvalue_4 (Math|Vector|MakeVector 0.0 0.0 _returnvalue_2))
  (bind _returnvalue_5 (Math|Vector|MakeVector 0.0 0.0 _returnvalue_3))
  (bind _outworldposition (Class|Tube|GetWorldOrientation _tube _returnvalue_4))
  (bind (_outworldposition_2 _outworldrotation) (Class|Tube|GetWorldOrientation _tube _returnvalue_5))
  (bind _returnvalue_6 (- _outworldposition_2 _returnvalue))
  (bind _returnvalue_7 (- _outworldposition _returnvalue))
  (bind _returnvalue_8 (Math|Vector|Normalize _returnvalue_7))
  (bind _returnvalue_9 (- _returnvalue _returnvalue_6))
  (bind _returnvalue_10 (Math|Vector|Normalize _returnvalue_6))
  (bind _returnvalue_11 (Math|Vector|DotProduct _returnvalue_10 _returnvalue_8))
  (bind _returnvalue_12 (Math|Float|Absolute(Float) _returnvalue_11))
  (bind _returnvalue_13 (- 1.0 _returnvalue_12))
  (bind _returnvalue_14 (* _returnvalue_13 0.3))
  (bind _returnvalue_15 (Math|Vector|Lerp(Vector) _outworldposition _returnvalue_9 _returnvalue_14))
  (Transformation|SetWorldLocationAndRotation (Variables|Default|GetCameraTo) _outworldposition_2 _outworldrotation false false)
  (Transformation|SetWorldLocationAndRotation (Variables|Default|GetCameraFrom) _returnvalue_15 (Class|JonBPExtension|LookatwithUp _returnvalue_15 _outworldposition_2 (Math|Vector|GetUpVector (.outWorldRotation (Class|Tube|GetWorldOrientation _tube _relativeposition)))) false false))

(fn ConstructionScript
  (Transformation|DetachFromComponent (Variables|Default|GetCameraFrom) "KeepRelative" "KeepRelative" "KeepRelative" true)
  (Transformation|DetachFromComponent (Variables|Default|GetCameraTo) "KeepRelative" "KeepRelative" "KeepRelative" true))