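; Single-player game mode for a tube crawl game, handling obstacle hits and checkpoints.
; On begin play it binds to the obstacle manager's hit event and the checkpoint manager's reached event, then places the first checkpoint.
; Hit obstacles are destroyed.
; Each reached checkpoint spawns the next one ahead of the crawler's relative Z by checkpoint time multiplied by crawler speed.
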(event Custom|Event%20Obstacle%20Hit
  (params (TubeObstacle :type Tube%20Obstacle%20Object%20Reference) (TubeCrawler :type Tube%20Crawler%20Object%20Reference))
  (Actor|DestroyActor TubeObstacle))

(event Custom|Event%20Checkpoint%20Reached
  (params (CheckpointActor :type Actor%20Object%20Reference) (TubeCrawler :type Tube%20Crawler%20Object%20Reference))
  (bind _crawler (Variables|Default|Getcrawler))
  (Class|TubeCheckpointManager|SetCheckpoint (Variables|Default|GetcheckpointManager) (+ (.Z (Math|Vector|BreakVector (Variables|/Script/Sadsads.TubeCrawler|GetrelativePosition _crawler))) (* (Variables|Default|GetcheckpointTime) (Variables|/Script/Sadsads.TubeCrawler|Getspeed _crawler)))))

(event EventBeginPlay
  (bind _crawler (Variables|Default|Getcrawler))
  (|CallParentFunction)
  (EventDispatchers|BindEventtoObstacleHitEvent (Variables|Default|GetobstacleManager) (delegate Custom|Event%20Obstacle%20Hit))
  (EventDispatchers|AssignCheckpointReachedEvent (Variables|Default|GetcheckpointManager) (delegate Custom|Event%20Checkpoint%20Reached))
  (Class|TubeCheckpointManager|SetCheckpoint (Variables|Default|GetcheckpointManager) (+ (.Z (Math|Vector|BreakVector (Variables|/Script/Sadsads.TubeCrawler|GetrelativePosition _crawler))) (* (Variables|Default|GetcheckpointTime) (Variables|/Script/Sadsads.TubeCrawler|Getspeed _crawler)))))

(event EventTick
  (params (DeltaSeconds :type Float%20%28single-precision%29)))

(fn ConstructionScript)